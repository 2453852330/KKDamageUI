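; BP_KKDamageUI is an actor that displays a damage number in the game through a widget component.
; On BeginPlay it casts the component's widget to UI_KKDamageUI and initializes it with the damage value as text and the damage color at full alpha.
; It binds to the widget's animation-finish event, intended to destroy the actor once the animation completes.
; The author notes that the widget can be swapped for a custom one.
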(event `self.ReceiveBeginPlay`
  (bind (_r _g _b) (`KismetMathLibrary.BreakColor` (`self.DamageColor`)))
  ;[0 1 1] 可以将此处修改为你的自定义Widget;你需要自行处理Actor的销毁,这里是在Widget动画播放完成时销毁;
  ; you can change bp to use your custom widget; you have to handle with the actor's destory which i destory on the widget's animation finish;
  (bind _asui_kkdamage_ui (cast `/KKDamageUI/UI_KKDamageUI` (`WidgetComponent.GetUserWidgetObject` (`self.Widget`))))
  (`/KKDamageUI/UI_KKDamageUI.KKInit` _asui_kkdamage_ui (`KismetTextLibrary.Conv_DoubleToText` (`self.DamageValue`) "HalfToEven" false false 1 324 0 0) (make `LinearColor` _r _g _b 1.0))
  (add `/KKDamageUI/UI_KKDamageUI.KKOnAnimationFinish` _asui_kkdamage_ui (`|CreateDelegate` :!event `DG_OnAnimationPlayFinish`)))

(fn `DG_OnAnimationPlayFinish`
  (`self.K2_DestroyActor`))

(fn `UserConstructionScript`)