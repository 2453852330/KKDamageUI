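; Player controller for demonstrating damage-number UI, which adds a crosshair widget for the local player.
; Left mouse click calls a server event that, despite its line-trace name, runs a large multi-sphere trace around the controlled pawn.
; Each hit actor tagged "A" gets a random damage value shown at its impact point via the character's KKDamageUI, with multicast enabled.
; No actual damage is applied.
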(event `self.ReceiveBeginPlay`
  ;[1 0.9141 0] create widget on local player client
  (if (`self.IsLocalPlayerController`)
    (bind _returnvalue (`|CreateWidget` "/KKDamageUI/Gameplay/UI_Crosshair.UI_Crosshair_C" self))
    (`UserWidget.AddToViewport` _returnvalue 0)))

(event `Key|LeftMouseButton`
  (params (Key :type "Key Structure"))
  ;[1 0.02344 0] rpc call on server
  (:`Pressed`
    (`self.Server_LineTraceAndDamageItem`)))

(event `Server_LineTraceAndDamageItem`
  (bind _returnvalue (`self.K2_GetActorLocation` (`self.K2_GetPawn`)))
  ;[0.8281 0 1] server :  cause damage
  (bind (_outhits _returnvalue_2) (`KismetSystemLibrary.SphereTraceMulti` _returnvalue (+ _returnvalue (0.0 0.0 10.0)) 1000.0 "TraceTypeQuery1" true))
  (if _returnvalue_2
    (for _array_element _outhits
      (bind (_bblockinghit _binitialoverlap _time _distance _location _impactpoint _normal _impactnormal _physmat _hitactor) (`GameplayStatics.BreakHitResult` _array_element))
      (if (`self.ActorHasTag` _hitactor "A")
        (bind _asbp_character_damage_ui (cast `/KKDamageUI/Gameplay/BP_Character_DamageUI` (`self.K2_GetPawn`)))
        (`KKDamageUIComponent.KKAddDamageUI` (`/KKDamageUI/Gameplay/BP_Character_DamageUI.KKDamageUI` _asbp_character_damage_ui) _impactpoint (`KismetMathLibrary.RandomFloatInRange` 0.0 999.0) true)))))

(fn `UserConstructionScript`)